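; Light_BP is a toggleable point light actor that exposes a ToggleLight event.
; ToggleLight flips IsOn, applies it to the PointLight's visibility, then sets the light color to NewColor on every toggle.
; The construction script applies IsOn to the light's visibility so the initial state matches the variable, but it leaves the color untouched until the first toggle.
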(event EventBeginPlay)

(event Collision|EventActorBeginOverlap
  (params (OtherActor :type Actor%20Object%20Reference)))

(event EventTick
  (params (DeltaSeconds :type Float%20%28single-precision%29)))

(event EventToggleLight
  (bind _output_get (Variables|Default|SetIsOn? (not (Variables|Default|GetIsOn?))))
  (Rendering|SetVisibility (Variables|Default|GetPointLight) _output_get false)
  (Rendering|Components|Light|SetLightColor (Variables|Default|GetPointLight) (Variables|Default|GetNewColor) true))

(fn ConstructionScript
  (Rendering|SetVisibility (Variables|Default|GetPointLight) (Variables|Default|GetIsOn?) false))