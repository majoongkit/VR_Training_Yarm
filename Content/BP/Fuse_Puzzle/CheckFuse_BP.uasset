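; CheckFuse_BP is a fuse puzzle checker that tracks Fuse actors entering and leaving its collision component.
; It caches the player's VRPawnPhysics on BeginPlay and increments that pawn's Fuse count on begin overlap, decrementing it on end overlap.
; An insertion also sets the pawn's current mission from Setmission, with a DoOnce and delayed reset throttling repeat counts.
; Removal has no such cooldown, and both changes print the count.
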(event OnComponentBeginOverlap(CollisionComponent)
  (params (OverlappedComponent :type Primitive%20Component%20Object%20Reference) (OtherActor :type Actor%20Object%20Reference) (OtherComp :type Primitive%20Component%20Object%20Reference) (OtherBodyIndex :type Integer) (bFromSweep :type Boolean) (SweepResult :type Hit%20Result%20Structure%20%28by%20ref%29))
  (bind _as_vrpawn_physics (Variables|Default|GetAs%20VRPawn%20Physics))
  (Utilities|Casting|CastToFuse OtherActor)
  (Utilities|FlowControl|DoOnce false :!label _label
    (:Completed
      (bind _output_get (Variables|/Game/VRTemplate/Blueprints/VRPawnPhysics.VRPawnPhysics_C|SetFuse _as_vrpawn_physics (+ (Variables|/Game/VRTemplate/Blueprints/VRPawnPhysics.VRPawnPhysics_C|GetFuse _as_vrpawn_physics) 1)))
      (Development|PrintString (Utilities|String|ToString(Integer) _output_get))
      (Variables|/Game/VRTemplate/Blueprints/VRPawnPhysics.VRPawnPhysics_C|Setcurrentmission _as_vrpawn_physics (Variables|Default|Getsetmission))
      (Utilities|FlowControl|Delay 1e+01)
      (goto _label Reset))))

(event OnComponentEndOverlap(CollisionComponent)
  (params (OverlappedComponent :type Primitive%20Component%20Object%20Reference) (OtherActor :type Actor%20Object%20Reference) (OtherComp :type Primitive%20Component%20Object%20Reference) (OtherBodyIndex :type Integer))
  (bind _as_vrpawn_physics (Variables|Default|GetAs%20VRPawn%20Physics))
  (Utilities|Casting|CastToFuse OtherActor)
  (Utilities|FlowControl|DoOnce false :!label _label
    (:Completed
      (bind _output_get (Variables|/Game/VRTemplate/Blueprints/VRPawnPhysics.VRPawnPhysics_C|SetFuse _as_vrpawn_physics (- (Variables|/Game/VRTemplate/Blueprints/VRPawnPhysics.VRPawnPhysics_C|GetFuse _as_vrpawn_physics) 1)))
      (Development|PrintString (Utilities|String|ToString(Integer) _output_get))
      (goto _label Reset))))

(event Custom|Overlap
  (bind _as_vrpawn_physics (Variables|Default|GetAs%20VRPawn%20Physics))
  (Utilities|FlowControl|DoOnce false :!label _label
    (:Completed
      (bind _output_get (Variables|/Game/VRTemplate/Blueprints/VRPawnPhysics.VRPawnPhysics_C|SetFuse _as_vrpawn_physics (+ (Variables|/Game/VRTemplate/Blueprints/VRPawnPhysics.VRPawnPhysics_C|GetFuse _as_vrpawn_physics) 1)))
      (Development|PrintString (Utilities|String|ToString(Integer) _output_get))
      (Variables|/Game/VRTemplate/Blueprints/VRPawnPhysics.VRPawnPhysics_C|Setcurrentmission _as_vrpawn_physics (Variables|Default|Getsetmission))
      (Utilities|FlowControl|Delay 1e+01)
      (goto _label Reset))))

(event EventBeginPlay
  (bind _asvrpawn_physics (Utilities|Casting|CastToVRPawnPhysics (Game|GetPlayerCharacter 0)))
  (Variables|Default|SetAs%20VRPawn%20Physics _asvrpawn_physics))

(fn ConstructionScript)