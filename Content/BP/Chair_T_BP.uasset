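; Triggered chair prop for VR that slides and then rotates with a crash sound.
; The first VRPawnPhysics overlap of the box, or any Play call, starts the slide sound and a timeline that offsets the chair from its captured relative location.
; That timeline's first update also schedules, once only, a short delay before the crash and a second timeline, which derives rotation from its vector plus that saved location.
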(event OnComponentBeginOverlap(Box)
  (params (OverlappedComponent :type Primitive%20Component%20Object%20Reference) (OtherActor :type Actor%20Object%20Reference) (OtherComp :type Primitive%20Component%20Object%20Reference) (OtherBodyIndex :type Integer) (bFromSweep :type Boolean) (SweepResult :type Hit%20Result%20Structure%20%28by%20ref%29))
  (Utilities|Casting|CastToVRPawnPhysics OtherActor)
  (Utilities|FlowControl|DoOnce false
    (:Completed
      (Variables|Default|SetDirection (Variables|/Script/Engine.SceneComponent|GetRelativeLocation (Variables|Default|GetChair)))
      (Audio|PlaySound2D "/Game/Sound/ChairSlide_Cue.ChairSlide_Cue" 1.0 1.0 0.0 0 0)
      (bind _movemont (Timeline|Timeline Play)
        (:Update
          (Transformation|SetRelativeLocation (Variables|Default|GetChair) (+ _movemont (Variables|Default|GetDirection)) false false)
          (Utilities|FlowControl|DoOnce false
            (:Completed
              (Utilities|FlowControl|Delay 0.2)
              (Audio|PlaySound2D "/Game/Sound/crash.crash" 1.0 1.0 0.0 0 0)
              (bind _movemont_2 (Timeline|Timeline_0 Play)
                (:Update
                  (Transformation|SetRelativeRotation (Variables|Default|GetChair) (Math|Conversions|RotationFromXVector (+ _movemont_2 (Variables|Default|GetDirection))) false false))))))))))

(event Custom|Play
  (Variables|Default|SetDirection (Variables|/Script/Engine.SceneComponent|GetRelativeLocation (Variables|Default|GetChair)))
  (Audio|PlaySound2D "/Game/Sound/ChairSlide_Cue.ChairSlide_Cue" 1.0 1.0 0.0 0 0)
  (bind _movemont (Timeline|Timeline Play)
    (:Update
      (Transformation|SetRelativeLocation (Variables|Default|GetChair) (+ _movemont (Variables|Default|GetDirection)) false false)
      (Utilities|FlowControl|DoOnce false
        (:Completed
          (Utilities|FlowControl|Delay 0.2)
          (Audio|PlaySound2D "/Game/Sound/crash.crash" 1.0 1.0 0.0 0 0)
          (bind _movemont_2 (Timeline|Timeline_0 Play)
            (:Update
              (Transformation|SetRelativeRotation (Variables|Default|GetChair) (Math|Conversions|RotationFromXVector (+ _movemont_2 (Variables|Default|GetDirection))) false false))))))))

(event EventBeginPlay)

(event Collision|EventActorBeginOverlap
  (params (OtherActor :type Actor%20Object%20Reference)))

(event EventTick
  (params (DeltaSeconds :type Float%20%28single-precision%29)))

(fn ConstructionScript)