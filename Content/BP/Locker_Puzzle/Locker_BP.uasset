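; VR puzzle locker with a hinged door that motion controllers can grab and swing once its KeyHole is unlocked.
; Grab stores a controller within the Sphere's radius as Hand, and Release clears it.
; Tick locks the door only while it is shut and the KeyHole is not unlocked.
; An unlocked door's world yaw follows the hand via look-at, clamped to a half-turn range, and snaps shut when released nearly closed.
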(event EventBeginPlay)

(event EventGrab
  (params (MotionController :type Motion%20Controller%20Component%20Object%20Reference))
  (bind _sphere (Variables|Default|GetSphere))
  (if (Utilities|Operators|EqualEqual (Transformation|GetWorldLocation MotionController) (Transformation|GetWorldLocation _sphere) (Variables|/Script/Engine.SphereComponent|GetSphereRadius _sphere))
    (Variables|Default|SetHand MotionController)))

(event EventTick
  (params (DeltaSeconds :type Float%20%28single-precision%29))
  (bind _hand (Variables|Default|GetHand))
  (bind _lockerdoor (Variables|Default|GetLockerDoor))
  (Utilities|FlowControl|Sequence
    (:then_0
      ;[1 0 0.001265] Locked
      (if (and (not (Variables|/Game/BP/Locker_Puzzle/KeyHole_BP.KeyHole_BP_C|GetUnlocked (Variables|Default|GetKeyHole))) (Math|Float|NearlyEqual(Float) (.yaw (Transformation|GetWorldRotation (Variables|Default|GetLockerDoor))) 0.0 1e-06))
        (Variables|Default|SetLocked true)
        (else
          (Variables|Default|SetLocked false))))
    (:then_1
      ;[0 1 0.0581] Set door rotation
      (if (not (Variables|Default|GetLocked))
        (Utilities|IsValid _hand
          (:Is%20Valid
            (Transformation|SetWorldRotation _lockerdoor (Math|Rotator|MakeRotator 0.0 0.0 (Math|Float|ClampAngle (- (.yaw (Math|Rotator|FindLookatRotation (Transformation|GetWorldLocation _hand) (Transformation|GetWorldLocation _lockerdoor))) 9e+01) -9e+01 9e+01)) false false))
          (:Is%20Not%20Valid
            (if (Math|Float|NearlyEqual(Float) (.yaw (Transformation|GetWorldRotation _lockerdoor)) 0.0 1e+01)
              (Transformation|SetWorldRotation _lockerdoor "0, 0, 0" false false))))))))

(event EventRelease
  (params (Motion%20controller :type Motion%20Controller%20Component%20Object%20Reference))
  (if (== Motion%20controller (Variables|Default|GetHand))
    (Variables|Default|SetHand 0)))

(fn ConstructionScript)