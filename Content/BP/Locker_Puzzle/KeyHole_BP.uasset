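; VR keyhole for a locker puzzle that guides a KeyLocker_BP key along a slot and tracks an Unlocked state.
; A held key slides on the segment between two spline points, snapping back to the motion controller at the start.
; A released key locks and attaches near the end, otherwise it simulates physics.
; Without a key, Tick sphere-checks the start and detaches the first key found, but never assigns Key.
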(event EventBeginPlay
  (bind _spline (Variables|Default|GetSpline))
  (Variables|Default|SetStartPoint (Spline|GetLocationatSplinePoint _spline 1 "Local"))
  (Variables|Default|SetEndPoint (Spline|GetLocationatSplinePoint _spline 0 "Local")))

(event EventTick
  (params (DeltaSeconds :type Float%20%28single-precision%29))
  (Utilities|IsValid (Variables|Default|GetKey)
    (:Is%20Valid
      (Utilities|IsValid (Variables|/Game/BP/Locker_Puzzle/KeyLocker_BP.KeyLocker_BP_C|GetMotion%20Controller (Variables|Default|GetKey))
        (:Is%20Valid
          ;[1 0.3137 0.8876] Keyslide
          (Transformation|SetActorLocation (Variables|Default|GetKey) (Math|Vector|FindClosestPointonSegment (Transformation|GetWorldLocation (Variables|/Game/BP/Locker_Puzzle/KeyLocker_BP.KeyLocker_BP_C|GetMotion%20Controller (Variables|Default|GetKey))) (Variables|Default|GetStartPoint) (Variables|Default|GetEndPoint)) false false)
          (if (Utilities|Operators|EqualEqual (Transformation|GetActorLocation (Variables|Default|GetKey)) (Variables|Default|GetStartPoint) 1e+01)
            (Transformation|AttachComponentToComponent (Variables|Default|GetKey) (Variables|/Game/BP/Locker_Puzzle/KeyLocker_BP.KeyLocker_BP_C|GetMotion%20Controller (Variables|Default|GetKey)) "None" "SnapToTarget" "SnapToTarget" "KeepWorld" true)
            (Variables|Default|SetKey 0)
            (Variables|Default|SetUnlocked false)))
        (:Is%20Not%20Valid
          ;[0.3117 1 0.3678] attachKey
          (if (Utilities|Operators|EqualEqual (Transformation|GetActorLocation (Variables|Default|GetKey)) (Variables|Default|GetEndPoint) 3e+01)
            (Variables|Default|SetUnlocked true)
            (Transformation|SetActorLocation (Variables|Default|GetKey) "0, 0, 0" false false)
            (Transformation|AttachActorToActor (Variables|Default|GetKey) self "None" "KeepWorld" "KeepWorld" "KeepWorld" true)
            (Physics|SetSimulatePhysics (Variables|/Game/BP/Locker_Puzzle/KeyLocker_BP.KeyLocker_BP_C|GetKeyLocker (Variables|Default|GetKey)) false)
            (else
              (Physics|SetSimulatePhysics (Variables|/Game/BP/Locker_Puzzle/KeyLocker_BP.KeyLocker_BP_C|GetKeyLocker (Variables|Default|GetKey)) true))))))
    (:Is%20Not%20Valid
      ;[1 0.2912 0] Detach Key
      (bind _outactors (Collision|SphereOverlapActors (Variables|Default|GetStartPoint) 2e+01 (Utilities|Array|MakeArray "ObjectTypeQuery1") 0))
      (bind _array_element (Utilities|Array|ForEachLoopwithBreak _outactors :!label _label)
        (:LoopBody
          (bind _askey_locker_bp (Utilities|Casting|CastToKeyLocker_BP _array_element))
          (bind _output_get (Variables|Default|SetAs%20Key%20Locker%20BP _askey_locker_bp))
          (Transformation|DetachFromActor _output_get "KeepWorld" "KeepWorld" "KeepRelative")
          (goto _label Break))))))

(fn ConstructionScript)