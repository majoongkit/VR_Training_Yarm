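; KeyLocker_BP is a VR grabbable key for the locker puzzle.
; It plays a key jingle at the key's location on BeginPlay.
; When GrabComponent fires OnGrabbed, it writes SetMission to the VR pawn's current mission and clears sound mix modifiers.
; Older Grab/Release events remain, toggling physics and attaching to the motion controller, with Release re-attaching at world transform rather than detaching.
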(event OnGrabbed(GrabComponent)
  (params (Motion%20Controller :type Motion%20Controller%20Component%20Object%20Reference))
  (bind _asvrpawn_physics (Utilities|Casting|CastToVRPawnPhysics (Game|Player|GetPlayerPawn 0)))
  (Variables|/Game/VRTemplate/Blueprints/VRPawnPhysics.VRPawnPhysics_C|Setcurrentmission _asvrpawn_physics (Variables|Default|Getset%20mission))
  (Class|GameplayStatics|ClearSoundMixModifiers))

(event EventBeginPlay
  (Audio|PlaySoundatLocation "/Game/Sound/key-jingle-36785_Cue.key-jingle-36785_Cue" (Transformation|GetWorldLocation (Variables|Default|GetKeyLocker)) "0, 0, 0" 1.0 1.0 0.0 0 0 0 0))

(event Collision|EventActorBeginOverlap
  (params (OtherActor :type Actor%20Object%20Reference)))

(event EventTick
  (params (DeltaSeconds :type Float%20%28single-precision%29)))

(event EventGrab
  (params (MotionController :type Motion%20Controller%20Component%20Object%20Reference))
  ;[1 1 1] Old BP
  (bind _output_get (Variables|Default|SetMotion%20Controller MotionController))
  (Transformation|AttachComponentToComponent _output_get "None" "SnapToTarget" "SnapToTarget" "KeepWorld" true)
  (Physics|SetSimulatePhysics (Variables|Default|GetKeyLocker) false))

(event EventRelease
  (params (Motion%20controller :type Motion%20Controller%20Component%20Object%20Reference))
  ;[1 1 1] Old BP
  (bind _output_get (Variables|Default|SetMotion%20Controller_0 Motion%20controller))
  (Transformation|AttachComponentToComponent _output_get "None" "KeepWorld" "KeepWorld" "KeepWorld" true)
  (Physics|SetSimulatePhysics (Variables|Default|GetKeyLocker) true))

(fn ConstructionScript)