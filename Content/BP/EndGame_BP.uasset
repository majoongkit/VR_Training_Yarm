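; End-game trigger actor that delivers a scream scare and then quits the game.
; When VRPawnPhysics overlaps the Box, or the End event is called, it instantly snaps components H1 to H4 to fixed relative positions.
; All four moves feed a shared tail that plays the scream in 2D on each pass, then quits after a short Delay.
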(event OnComponentBeginOverlap(Box)
  (params (OverlappedComponent :type Primitive%20Component%20Object%20Reference) (OtherActor :type Actor%20Object%20Reference) (OtherComp :type Primitive%20Component%20Object%20Reference) (OtherBodyIndex :type Integer) (bFromSweep :type Boolean) (SweepResult :type Hit%20Result%20Structure%20%28by%20ref%29))
  (Utilities|Casting|CastToVRPawnPhysics OtherActor)
  (Utilities|FlowControl|Sequence
    (:then_0
      (Transformation|SetRelativeLocation (Variables|Default|GetH1) "50.702118,-36.962135,0.000002" false false))
    (:then_1
      (Transformation|SetRelativeLocation (Variables|Default|GetH2) "98.475499,11.257556,-0.000011" false false))
    (:then_2
      (Transformation|SetRelativeLocation (Variables|Default|GetH3) "-23.709065,-44.100986,-0.000002" false false))
    (:then_3
      (Transformation|SetRelativeLocation (Variables|Default|GetH4) "-80.023807,11.000000,0.000000" false false)))
  (Utilities|FlowControl|Sequence
    (:then_0
      (Audio|PlaySound2D "/Game/Sound/scream_Cue.scream_Cue" 1.0 1.0 0.0 0 0))
    (:then_1
      (Utilities|FlowControl|Delay 3.0)
      (Game|QuitGame 0 "Quit" false))))

(event Custom|End
  (Utilities|FlowControl|Sequence
    (:then_0
      (Transformation|SetRelativeLocation (Variables|Default|GetH1) "50.702118,-36.962135,0.000002" false false))
    (:then_1
      (Transformation|SetRelativeLocation (Variables|Default|GetH2) "98.475499,11.257556,-0.000011" false false))
    (:then_2
      (Transformation|SetRelativeLocation (Variables|Default|GetH3) "-23.709065,-44.100986,-0.000002" false false))
    (:then_3
      (Transformation|SetRelativeLocation (Variables|Default|GetH4) "-80.023807,11.000000,0.000000" false false)))
  (Utilities|FlowControl|Sequence
    (:then_0
      (Audio|PlaySound2D "/Game/Sound/scream_Cue.scream_Cue" 1.0 1.0 0.0 0 0))
    (:then_1
      (Utilities|FlowControl|Delay 3.0)
      (Game|QuitGame 0 "Quit" false))))

(event EventBeginPlay)

(event Collision|EventActorBeginOverlap
  (params (OtherActor :type Actor%20Object%20Reference)))

(event EventTick
  (params (DeltaSeconds :type Float%20%28single-precision%29)))

(fn ConstructionScript)